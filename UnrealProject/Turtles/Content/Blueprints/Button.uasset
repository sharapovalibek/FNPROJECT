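; Interactable button actor that spawns a turtle through a linked Socket when used.
; Interact checks that the Socket is valid, plays the press animation, then calls SpawnTurtle on it.
; The press tints a construction-time dynamic material green while a timeline lerps the mesh between its cached relative location and a fixed offset, restoring the original color when finished.
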(event Custom|PlayInteractionAnimation
  (Rendering|Material|SetVectorParameterValue (Variables|Default|GetButtonMat) "Color" "(R=0.000000,G=0.625000,B=0.069524,A=1.000000)" :!class /Script/Engine.MaterialInstanceDynamic)
  (bind _alpha (Timeline|Timeline_ButtonMove PlayFromStart)
    (:Update
      (Transformation|SetRelativeLocation (Variables|Default|GetButton) (Math|Vector|Lerp(Vector) (Variables|Default|GetCachedRelativeLocation) "0, 0,46.000000" _alpha) false false))
    (:Finished
      (Rendering|Material|SetVectorParameterValue (Variables|Default|GetButtonMat) "Color" (Variables|Default|GetBaseColor) :!class /Script/Engine.MaterialInstanceDynamic))))

(event EventBeginPlay
  (Variables|Default|SetCachedRelativeLocation (Variables|/Script/Engine.SceneComponent|GetRelativeLocation (Variables|Default|GetButton)))
  (bind _returnvalue (Rendering|Material|GetVectorParameterValue (Variables|Default|GetButtonMat) "Color" :!class /Script/Engine.MaterialInstanceDynamic))
  (Variables|Default|SetBaseColor _returnvalue))

(event Collision|EventActorBeginOverlap
  (params (OtherActor :type Actor%20Object%20Reference)))

(event EventTick
  (params (DeltaSeconds :type Float%20%28single-precision%29)))

(event EventInteract
  (bind _socket (Variables|Default|GetSocket)
    (:then
      (CallFunction|PlayInteractionAnimation)
      (Default|SpawnTurtle _socket))
    (:else)))

(fn ConstructionScript
  (bind _returnvalue (Rendering|Material|CreateDynamicMaterialInstance (Variables|Default|GetButton) 0 "/Game/Materials/Button/M_Button_Inst.M_Button_Inst" "None" :!class /Script/Engine.PrimitiveComponent))
  (Variables|Default|SetButtonMat _returnvalue))