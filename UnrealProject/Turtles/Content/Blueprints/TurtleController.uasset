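; AI controller that starts the behavior tree for a Turtle pawn.
; On BeginPlay it waits briefly, then casts the controlled pawn to Turtle and runs the behavior tree stored on that pawn.
; It then seeds the Blackboard with the Turtle's Destination and records its current location as SpawnPoint.
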(event EventBeginPlay
  (bind _blackboard (Variables|Default|GetBlackboard))
  (Utilities|FlowControl|Delay 0.2) ; Controller doesn't exist yet
  (bind _asturtle (Utilities|Casting|CastToTurtle (Pawn|GetControlledPawn)))
  (AI|RunBehaviorTree (Variables|/Game/Blueprints/Turtle.Turtle_C|GetBehaviourTree _asturtle))
  (AI|Components|Blackboard|SetValueasVector _blackboard (Utilities|Name|MakeLiteralName "Destination") (Variables|/Game/Blueprints/Turtle.Turtle_C|GetDestination _asturtle))
  (AI|Components|Blackboard|SetValueasVector _blackboard (Utilities|Name|MakeLiteralName "SpawnPoint") (Transformation|GetActorLocation _asturtle)))

(fn ConstructionScript)